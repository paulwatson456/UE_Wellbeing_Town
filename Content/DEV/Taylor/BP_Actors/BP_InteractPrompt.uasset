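; Interaction prompt actor with a widget that shows available interaction icons and passes F presses to a parent BP_NPCTest to continue dialogue.
; BeginPlay and UpdateInteractions fill the widget's wrap box from the Interactions list, adding Inquire only if the player holds the "Inquire Ability" quest reward.
; ShowPrompt fades the icons in via a timeline when CanInteract is set, then reverses after a short delay.
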(event Custom|UpdateInteractions
  (bind _aswi_interaction_box (Utilities|Casting|CastToWI_InteractionBox (UserInterface|GetWidget (Variables|Default|GetWidget1))))
  (Widget|Panel|ClearChildren (Variables|/Game/DEV/Taylor/Widgets/WI_InteractionBox.WI_InteractionBox_C|GetWrapBox_0 _aswi_interaction_box))
  (bind _asbp_player (Utilities|Casting|CastToBP_Player (Game|GetPlayerCharacter 0)))
  (for _array_element (Variables|Default|GetInteractions)
    (if (== _array_element "/Game/DEV/Taylor/Widgets/Images/Inquire.Inquire")
      (if (Utilities|Array|ContainsItem (Variables|/Game/DEV/Taylor/BP_CC/BP_Player.BP_Player_C|GetQuestRewards _asbp_player) "Inquire Ability")
        (bind _aswi_interaction_box_2 (Utilities|Casting|CastToWI_InteractionBox (UserInterface|GetWidget (Variables|Default|GetWidget1)) :!label _label))
        (bind _returnvalue (UserInterface|CreateWidget "/Game/DEV/Taylor/Widgets/WI_Interact.WI_Interact_C"))
        (Class|Image|SetBrush (Variables|/Game/DEV/Taylor/Widgets/WI_Interact.WI_Interact_C|GetImage_0 _returnvalue) (Utilities|Struct|MakeSlateBrush "Image" "NoTile" "NoMirror" "(X=32.000000,Y=32.000000)" "(Left=0.000000,Top=0.000000,Right=0.000000,Bottom=0.000000)" "(SpecifiedColor=(R=1.000000,G=1.000000,B=1.000000,A=1.000000),ColorUseRule=UseColor_Specified)" "(CornerRadii=(X=0.000000,Y=0.000000,Z=0.000000,W=0.000000),Color=(SpecifiedColor=(R=0.000000,G=0.000000,B=0.000000,A=0.000000),ColorUseRule=UseColor_Specified),Width=0.000000,RoundingType=HalfHeightRadius,bUseBrushTransparency=False)" _array_element))
        (Widget|Panel|AddChild (Variables|/Game/DEV/Taylor/Widgets/WI_InteractionBox.WI_InteractionBox_C|GetWrapBox_0 _aswi_interaction_box_2) _returnvalue)
        (Widget|SetRenderOpacity (Variables|/Game/DEV/Taylor/Widgets/WI_InteractionBox.WI_InteractionBox_C|GetWrapBox_0 _aswi_interaction_box_2) 0.0))
      (else
        (goto _label)))))

(event Custom|ShowPrompt
  (bind _aswi_interaction_box (Utilities|Casting|CastToWI_InteractionBox (UserInterface|GetWidget (Variables|Default|GetWidget1))))
  (Utilities|FlowControl|Sequence
    (:then_0
      (if (Variables|Default|GetCanInteract?)
        (bind _newtrack_0 (Timeline|Timeline_0 Play)
          (:Update
            (Widget|SetRenderOpacity (Variables|/Game/DEV/Taylor/Widgets/WI_InteractionBox.WI_InteractionBox_C|GetWrapBox_0 _aswi_interaction_box) _newtrack_0)))
        (else
          (Timeline|Timeline_0 Reverse))))
    (:then_1
      (Utilities|FlowControl|Delay 0.2)
      (Timeline|Timeline_0 Reverse))))

(event EventBeginPlay
  (bind _asbp_player (Utilities|Casting|CastToBP_Player (Game|GetPlayerCharacter 0)))
  (for _array_element (Variables|Default|GetInteractions)
    (if (== _array_element "/Game/DEV/Taylor/Widgets/Images/Inquire.Inquire")
      (if (Utilities|Array|ContainsItem (Variables|/Game/DEV/Taylor/BP_CC/BP_Player.BP_Player_C|GetQuestRewards _asbp_player) "Inquire Ability")
        (bind _aswi_interaction_box (Utilities|Casting|CastToWI_InteractionBox (UserInterface|GetWidget (Variables|Default|GetWidget1)) :!label _label))
        (bind _returnvalue (UserInterface|CreateWidget "/Game/DEV/Taylor/Widgets/WI_Interact.WI_Interact_C"))
        (Class|Image|SetBrush (Variables|/Game/DEV/Taylor/Widgets/WI_Interact.WI_Interact_C|GetImage_0 _returnvalue) (Utilities|Struct|MakeSlateBrush "Image" "NoTile" "NoMirror" "(X=32.000000,Y=32.000000)" "(Left=0.000000,Top=0.000000,Right=0.000000,Bottom=0.000000)" "(SpecifiedColor=(R=1.000000,G=1.000000,B=1.000000,A=1.000000),ColorUseRule=UseColor_Specified)" "(CornerRadii=(X=0.000000,Y=0.000000,Z=0.000000,W=0.000000),Color=(SpecifiedColor=(R=0.000000,G=0.000000,B=0.000000,A=0.000000),ColorUseRule=UseColor_Specified),Width=0.000000,RoundingType=HalfHeightRadius,bUseBrushTransparency=False)" _array_element))
        (Widget|Panel|AddChild (Variables|/Game/DEV/Taylor/Widgets/WI_InteractionBox.WI_InteractionBox_C|GetWrapBox_0 _aswi_interaction_box) _returnvalue)
        (Widget|SetRenderOpacity (Variables|/Game/DEV/Taylor/Widgets/WI_InteractionBox.WI_InteractionBox_C|GetWrapBox_0 _aswi_interaction_box) 0.0))
      (else
        (goto _label)))))

(event Collision|EventActorBeginOverlap
  (params (OtherActor :type Actor%20Object%20Reference)))

(event EventTick
  (params (DeltaSeconds :type Float%20%28single-precision%29)))

(event Input|KeyboardEvents|F
  (params (Key :type Key%20Structure :default "None"))
  (:Pressed
    (bind _asbp_npctest (Utilities|Casting|CastToBP_NPCTest (Actor|GetAttachParentActor)))
    (Default|ContinueDialogue _asbp_npctest)))

(fn ConstructionScript)