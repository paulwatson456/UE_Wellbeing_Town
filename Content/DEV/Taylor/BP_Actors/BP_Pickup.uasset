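; BP_Pickup is a collectible item that the player picks up by overlapping its sphere.
; After a short delay on BeginPlay, it destroys itself if BP_Player already collected it, otherwise a timeline animates the cube's height and yaw.
; Overlap calls PickUp, plays a sound and destroys the actor, first recording any quest reward on the player and GI_WellnessTown.
; The construction script applies the configured mesh and materials.
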(event OnComponentBeginOverlap(Sphere)
  (params (OverlappedComponent :type Primitive%20Component%20Object%20Reference) (OtherActor :type Actor%20Object%20Reference) (OtherComp :type Primitive%20Component%20Object%20Reference) (OtherBodyIndex :type Integer) (bFromSweep :type Boolean) (SweepResult :type Hit%20Result%20Structure%20%28by%20ref%29))
  (bind _questreward (Variables|Default|GetQuestReward))
  (bind _returnvalue (Utilities|String|StringToName _questreward))
  (bind _asbp_player (Utilities|Casting|CastToBP_Player OtherActor))
  (if (Utilities|Array|IsEmpty _questreward)
    _
    (else
      (Utilities|Array|Add (Variables|/Game/DEV/Taylor/BP_CC/BP_Player.BP_Player_C|GetQuestRewards _asbp_player) _returnvalue)
      (bind _asgi_wellness_town (Utilities|Casting|CastToGI_WellnessTown (Game|GetGameInstance)))
      (Utilities|Array|Add (Variables|/Game/DEV/Taylor/GameInstance/GI_WellnessTown.GI_WellnessTown_C|GetQuest%20Rewards _asgi_wellness_town) _returnvalue)
      (Default|ItemGained _asbp_player (Variables|Default|GetQuestRewardIcon) _returnvalue)
      (Default|QuestRewardBenefits _asbp_player)))
  (Default|PickUp _asbp_player (Variables|Default|GetItem) (Variables|Default|GetObjectName))
  (Audio|PlaySoundatLocation (Variables|Default|GetSound) (Transformation|GetWorldLocation (Variables|Default|GetDefaultSceneRoot)) "0, 0, 0" 1.0 1.0 0.0 0 0 0 0)
  (Actor|DestroyActor))

(event EventBeginPlay
  (Utilities|FlowControl|Delay 0.21)
  (bind _asbp_player (Utilities|Casting|CastToBP_Player (Game|GetPlayerCharacter 0)))
  (if (Utilities|Array|ContainsItem (Variables|/Game/DEV/Taylor/BP_CC/BP_Player.BP_Player_C|GetCollectedItems _asbp_player) (Variables|Default|GetItem))
    (Actor|DestroyActor)
    (else
      (bind (_direction _newtrack_0 _newtrack_1) (Timeline|Timeline Play)
        (:Update
          (Transformation|SetRelativeLocationAndRotation (Variables|Default|GetCube) (Math|Vector|MakeVector 0.0 0.0 _newtrack_1) (Math|Rotator|MakeRotator 0.0 0.0 _newtrack_0) false false))))))

(event Collision|EventActorBeginOverlap
  (params (OtherActor :type Actor%20Object%20Reference)))

(event EventTick
  (params (DeltaSeconds :type Float%20%28single-precision%29)))

(fn ConstructionScript
  (if (Utilities|IsValid (Variables|Default|GetMesh))
    (Components|StaticMesh|SetStaticMesh (Variables|Default|GetCube) (Variables|Default|GetMesh))
    (for (_ _array_index) (Rendering|Material|GetMaterials (Variables|Default|GetCube))
      (Rendering|Material|SetMaterial (Variables|Default|GetCube) _array_index (Utilities|Array|Get(acopy) (Variables|Default|GetMaterial) _array_index)))))