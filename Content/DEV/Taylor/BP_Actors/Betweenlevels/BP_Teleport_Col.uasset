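; BP_Teleport_Col is a trigger volume, apparently for between-level transitions, with its box sized by BoxScale in the construction script.
; When BP_Player overlaps the box, it calls SetSpawnPos on every entry.
; A DoOnce then plays TriggerSound at the world origin, disables player input and clears CanInteract.
; The graph itself contains no teleport or level-load call.
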(event OnComponentBeginOverlap(Box)
  (params (OverlappedComponent :type Primitive%20Component%20Object%20Reference) (OtherActor :type Actor%20Object%20Reference) (OtherComp :type Primitive%20Component%20Object%20Reference) (OtherBodyIndex :type Integer) (bFromSweep :type Boolean) (SweepResult :type Hit%20Result%20Structure%20%28by%20ref%29))
  (bind _asbp_tp_interface_example (Utilities|Casting|CastToBP_Player OtherActor))
  (CallFunction|SetSpawnPos)
  (Utilities|FlowControl|DoOnce false
    (:Completed
      (Audio|PlaySoundatLocation (Variables|Default|GetTriggerSound) "0, 0, 0" "0, 0, 0" 1.0 1.0 0.0 0 0 0 0)
      (Input|DisableInput _asbp_tp_interface_example (Game|GetPlayerController 0))
      (Variables|/Game/DEV/Taylor/BP_CC/BP_Player.BP_Player_C|SetCanInteract? _asbp_tp_interface_example false))))

(event EventBeginPlay
  (|CallParentFunction) ; This node is disabled and will not be called.\nDrag off pins to build functionality.
)

(event Collision|EventActorBeginOverlap
  (params (OtherActor :type Actor%20Object%20Reference)))

(event EventTick
  (params (DeltaSeconds :type Float%20%28single-precision%29)))

(fn ConstructionScript
  (|CallParentFunction)
  (Transformation|SetRelativeScale3D (Variables|Default|GetBox) (Variables|Default|GetBoxScale)))