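; Level-transition door that walks the player into place, swings open and calls SetSpawnPos, closing again on BeginPlay when it matches the saved spawn.
; Interaction is blocked while carrying objects; timelines drive the player move and the flippable pivot rotation.
; On town nights general entry is disabled, and the player-house door swaps its prompt to Bed, leading to PlayerHouse with night and reflect flags set.
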(event Custom|OpenDoor
  (Audio|SpawnSoundAttached (Variables|Default|GetSound_DoorOpen) (Variables|Default|GetDoor) "None" "0, 0, 0" "0, 0, 0" "KeepRelativeOffset" false 1.0 1.0 0.0 "/Game/DEV/Taylor/Sound/DoorSoundAttenuation.DoorSoundAttenuation" 0)
  (bind _newtrack_0 (Timeline|Timeline Play)
    (:Update
      (if (Variables|Default|GetFlipRotation)
        (Transformation|SetRelativeRotation (Variables|Default|GetPivot) (Math|Rotator|MakeRotator 0.0 0.0 _newtrack_0) false false)
        (else
          (Transformation|SetRelativeRotation (Variables|Default|GetPivot) (Math|Rotator|MakeRotator 0.0 0.0 (* _newtrack_0 -1.0)) false false))))))

(event Custom|CloseDoor
  (Utilities|FlowControl|Sequence
    (:then_0
      (bind _newtrack_0 (Timeline|Timeline ReverseFromEnd)
        (:Update
          (if (Variables|Default|GetFlipRotation)
            (Transformation|SetRelativeRotation (Variables|Default|GetPivot) (Math|Rotator|MakeRotator 0.0 0.0 _newtrack_0) false false)
            (else
              (Transformation|SetRelativeRotation (Variables|Default|GetPivot) (Math|Rotator|MakeRotator 0.0 0.0 (* _newtrack_0 -1.0)) false false))))))
    (:then_1
      (Utilities|FlowControl|Delay 0.7)
      (Audio|SpawnSoundAttached (Variables|Default|GetSound_DoorClose) (Variables|Default|GetDoor) "None" "0, 0, 0" "0, 0, 0" "KeepRelativeOffset" false 1.0 1.0 0.0 "/Game/DEV/Taylor/Sound/DoorSoundAttenuation.DoorSoundAttenuation" 0))))

(event Custom|MovePlayer
  (bind _asbp_tp_interface_example (Utilities|Casting|CastToBP_TP_InterfaceExample (Game|GetPlayerCharacter 0)))
  (Input|DisableInput _asbp_tp_interface_example (Game|GetPlayerController 0))
  (Variables|/Game/DEV/Taylor/BP_CC/BP_TP_InterfaceExample.BP_TP_InterfaceExample_C|SetCanInteract? _asbp_tp_interface_example false)
  (bind _newtrack_0 (Timeline|Timeline_0 Play)
    (:Update
      (Transformation|SetWorldLocation (Variables|/Script/Engine.Character|GetCapsuleComponent _asbp_tp_interface_example) (Math|Vector|MakeVector (.x (Math|Vector|Lerp(Vector) (Transformation|GetWorldLocation (Variables|/Script/Engine.Character|GetCapsuleComponent _asbp_tp_interface_example)) (Transformation|GetWorldLocation (Variables|Default|GetArrow)) _newtrack_0)) (.y (Math|Vector|Lerp(Vector) (Transformation|GetWorldLocation (Variables|/Script/Engine.Character|GetCapsuleComponent _asbp_tp_interface_example)) (Transformation|GetWorldLocation (Variables|Default|GetArrow)) _newtrack_0)) (.Z (Math|Vector|BreakVector (Transformation|GetWorldLocation (Variables|/Script/Engine.Character|GetCapsuleComponent _asbp_tp_interface_example))))) false false)
      (Transformation|SetWorldRotation (Variables|/Script/Engine.Character|GetCapsuleComponent _asbp_tp_interface_example) (Math|Rotator|MakeRotator 0.0 0.0 (.yaw (Math|Rotator|FindLookatRotation (Transformation|GetWorldLocation (Variables|/Script/Engine.Character|GetCapsuleComponent _asbp_tp_interface_example)) (Transformation|GetWorldLocation (Variables|Default|GetDoor))))) false false))))

(event Custom|NightTime
  (if (Variables|Default|GetIsPlayerHouse)
    (Utilities|FlowControl|Delay 0.2)
    (bind _asgi_wellness_town (Utilities|Casting|CastToGI_WellnessTown (Game|GetGameInstance)))
    (if (Variables|/Game/DEV/Taylor/GameInstance/GI_WellnessTown.GI_WellnessTown_C|GetIsNightOnTownLevel? _asgi_wellness_town)
      (Utilities|FlowControl|DoOnce false
        (:Completed
          (bind _asbp_interact_prompt (Utilities|Casting|CastToBP_InteractPrompt (Variables|/Script/Engine.ChildActorComponent|GetChildActor (Variables|Default|GetBP_InteractPrompt))))
          (Utilities|Array|Clear (Variables|/Game/DEV/Taylor/BP_Actors/BP_InteractPrompt.BP_InteractPrompt_C|GetInteractions _asbp_interact_prompt))
          (Utilities|Array|Add (Variables|/Game/DEV/Taylor/BP_Actors/BP_InteractPrompt.BP_InteractPrompt_C|GetInteractions _asbp_interact_prompt) "/Game/DEV/Taylor/Widgets/Images/Bed.Bed")
          (Default|UpdateInteractions _asbp_interact_prompt))))))

(event EventBeginPlay
  (|CallParentFunction)
  (CallFunction|CanOpen?)
  (bind _asgi_wellness_town (Utilities|Casting|CastToGI_WellnessTown (Game|GetGameInstance)))
  (if (Variables|/Game/DEV/Taylor/GameInstance/GI_WellnessTown.GI_WellnessTown_C|GetIsNight? _asgi_wellness_town)
    (Collision|SetCollisionObjectType (Variables|Default|GetDoor) "ECC_WorldDynamic"))
  (if (Utilities|Enum|Equal(Enum) (Variables|/Game/DEV/Taylor/GameInstance/GI_WellnessTown.GI_WellnessTown_C|GetSpawn _asgi_wellness_town) (Variables|Default|GetDoorName))
    (CallFunction|CloseDoor))
  (if (Variables|Default|GetIsPlayerHouse)
    (Utilities|FlowControl|Delay 0.2)
    (bind _asgi_wellness_town_2 (Utilities|Casting|CastToGI_WellnessTown (Game|GetGameInstance)))
    (if (Variables|/Game/DEV/Taylor/GameInstance/GI_WellnessTown.GI_WellnessTown_C|GetIsNightOnTownLevel? _asgi_wellness_town_2)
      (Utilities|FlowControl|DoOnce false
        (:Completed
          (bind _asbp_interact_prompt (Utilities|Casting|CastToBP_InteractPrompt (Variables|/Script/Engine.ChildActorComponent|GetChildActor (Variables|Default|GetBP_InteractPrompt))))
          (Utilities|Array|Clear (Variables|/Game/DEV/Taylor/BP_Actors/BP_InteractPrompt.BP_InteractPrompt_C|GetInteractions _asbp_interact_prompt))
          (Utilities|Array|Add (Variables|/Game/DEV/Taylor/BP_Actors/BP_InteractPrompt.BP_InteractPrompt_C|GetInteractions _asbp_interact_prompt) "/Game/DEV/Taylor/Widgets/Images/Bed.Bed")
          (Default|UpdateInteractions _asbp_interact_prompt))))))

(event Collision|EventActorBeginOverlap
  (params (OtherActor :type Actor%20Object%20Reference)))

(event EventTick
  (params (DeltaSeconds :type Float%20%28single-precision%29)))

(event EventGeneralInteract
  (bind _asgi_wellness_town (Utilities|Casting|CastToGI_WellnessTown (Game|GetGameInstance)))
  (bind _asbp_tp_interface_example (Utilities|Casting|CastToBP_TP_InterfaceExample (Game|GetPlayerCharacter 0)))
  (if (not (or (Variables|/Game/DEV/Taylor/BP_CC/BP_TP_InterfaceExample.BP_TP_InterfaceExample_C|GetCarryingObject _asbp_tp_interface_example) (Variables|/Game/DEV/Taylor/GameInstance/GI_WellnessTown.GI_WellnessTown_C|GetIsNightOnTownLevel? _asgi_wellness_town)))
    (bind _asbp_interact_prompt (Utilities|Casting|CastToBP_InteractPrompt (Variables|/Script/Engine.ChildActorComponent|GetChildActor (Variables|Default|GetBP_InteractPrompt))))
    (Variables|/Game/DEV/Taylor/BP_Actors/BP_InteractPrompt.BP_InteractPrompt_C|SetCanInteract? _asbp_interact_prompt false)
    (CallFunction|MovePlayer)
    (CallFunction|OpenDoor)
    (Utilities|FlowControl|Delay 0.5)
    (CallFunction|SetSpawnPos)))

(event EventShowPrompt
  (bind _asbp_tp_interface_example (Utilities|Casting|CastToBP_TP_InterfaceExample (Game|GetPlayerCharacter 0)))
  (if (not (Variables|/Game/DEV/Taylor/BP_CC/BP_TP_InterfaceExample.BP_TP_InterfaceExample_C|GetCarryingObject _asbp_tp_interface_example))
    (bind _asbp_interact_prompt (Utilities|Casting|CastToBP_InteractPrompt (Variables|/Script/Engine.ChildActorComponent|GetChildActor (Variables|Default|GetBP_InteractPrompt))))
    (Default|ShowPrompt _asbp_interact_prompt)))

(event EventInteractE
  (bind _asbp_tp_interface_example (Utilities|Casting|CastToBP_TP_InterfaceExample (Game|GetPlayerCharacter 0)))
  (if (not (Variables|/Game/DEV/Taylor/BP_CC/BP_TP_InterfaceExample.BP_TP_InterfaceExample_C|GetCarryingObject _asbp_tp_interface_example))
    (bind _asgi_wellness_town (Utilities|Casting|CastToGI_WellnessTown (Game|GetGameInstance)))
    (if (Variables|/Game/DEV/Taylor/GameInstance/GI_WellnessTown.GI_WellnessTown_C|GetIsNightOnTownLevel? _asgi_wellness_town)
      (if (Variables|Default|GetIsPlayerHouse)
        (bind _asbp_interact_prompt (Utilities|Casting|CastToBP_InteractPrompt (Variables|/Script/Engine.ChildActorComponent|GetChildActor (Variables|Default|GetBP_InteractPrompt))))
        (Variables|/Game/DEV/Taylor/BP_Actors/BP_InteractPrompt.BP_InteractPrompt_C|SetCanInteract? _asbp_interact_prompt false)
        (CallFunction|MovePlayer)
        (CallFunction|OpenDoor)
        (Utilities|FlowControl|Delay 0.5)
        (Variables|Default|SetLevelName "PlayerHouse")
        (Variables|Default|SetDoorName "NewEnumerator5")
        (CallFunction|SetSpawnPos)
        (bind _asgi_wellness_town_2 (Utilities|Casting|CastToGI_WellnessTown (Game|GetGameInstance)))
        (Variables|/Game/DEV/Taylor/GameInstance/GI_WellnessTown.GI_WellnessTown_C|SetIsNight? _asgi_wellness_town_2 true)
        (Variables|/Game/DEV/Taylor/GameInstance/GI_WellnessTown.GI_WellnessTown_C|SetReflect? _asgi_wellness_town_2 true)))))

(fn ConstructionScript
  (|CallParentFunction))

(fn CanOpen?
  (if (not (Variables|Default|GetCanOpenDoor?))
    (Collision|SetCollisionObjectType (Variables|Default|GetDoor) "ECC_WorldDynamic")))