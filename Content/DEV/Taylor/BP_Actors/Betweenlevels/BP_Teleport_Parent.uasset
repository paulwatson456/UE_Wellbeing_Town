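; Parent level-transition door that moves the player between levels and places them at the matching door on arrival.
; SetSpawnPos fades screen and music, then saves quests, carried and loose pickups, rubbish, NPC wellness, collected items and music state to GI_WellnessTown before opening LevelName.
; It also stores DoorName, so on BeginPlay the door with that name teleports the player to its Arrow, whose offset the construction script sets.
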(event Custom|SetSpawnPos
  (CallFunction|OverlayFadein)
  (bind _asgi_wellness_town (Utilities|Casting|CastToGI_WellnessTown (Game|GetGameInstance)))
  (Audio|Components|Audio|AdjustVolume (Variables|/Game/DEV/Taylor/GameInstance/GI_WellnessTown.GI_WellnessTown_C|GetGameMusic _asgi_wellness_town) 1.0 0.5 "Linear" :!class /Script/Engine.AudioComponent)
  (Utilities|FlowControl|Delay (Variables|Default|GetOpenLevelDelay))
  (bind _asgi_wellness_town_2 (Utilities|Casting|CastToGI_WellnessTown (Game|GetGameInstance)))
  (Variables|/Game/DEV/Taylor/GameInstance/GI_WellnessTown.GI_WellnessTown_C|SetSpawn _asgi_wellness_town_2 (Variables|Default|GetDoorName))
  (bind _asgi_wellness_town_3 (Utilities|Casting|CastToGI_WellnessTown (Game|GetGameInstance)))
  (bind _asbp_tp_interface_example (Utilities|Casting|CastToBP_Player (Game|GetPlayerCharacter 0)))
  (for _array_element (Variables|/Game/DEV/Taylor/Quests/QuestComponent.QuestComponent_C|GetCurrentQuests (Variables|/Game/DEV/Taylor/BP_CC/BP_Player.BP_Player_C|GetQuestComponent _asbp_tp_interface_example))
    (Default|SaveQuestDetails _asgi_wellness_town_3 _array_element))
  (Default|SaveQuests _asgi_wellness_town_3)
  (bind _outactors (Actor|GetAllActorsOfClass "/Game/DEV/Taylor/BP_Actors/BinObjects/BP_PickupParent.BP_PickupParent_C"))
  (bind _output_get (Variables|/Game/DEV/Taylor/GameInstance/GI_WellnessTown.GI_WellnessTown_C|SetBag _asgi_wellness_town_3 (Variables|/Game/DEV/Taylor/BP_CC/BP_Player.BP_Player_C|GetCarryingObject _asbp_tp_interface_example)))
  (if _output_get
    (Variables|/Game/DEV/Taylor/GameInstance/GI_WellnessTown.GI_WellnessTown_C|SetCarrying _asgi_wellness_town_3 (Variables|/Game/DEV/Taylor/BP_Actors/BinObjects/BP_PickupParent.BP_PickupParent_C|GetObjectClass (Variables|/Game/DEV/Taylor/BP_CC/BP_Player.BP_Player_C|GetBag _asbp_tp_interface_example)))
    (Utilities|Array|RemoveItem _outactors (Variables|/Game/DEV/Taylor/BP_CC/BP_Player.BP_Player_C|GetBag _asbp_tp_interface_example)))
  (bind _returnvalue (Game|GetCurrentLevelName true))
  (if (Utilities|Array|IsNotEmpty _outactors)
    (for _array_element_2 _outactors
      (Default|SaveObjects _asgi_wellness_town_3 (Transformation|GetWorldRotation (Variables|/Game/DEV/Taylor/BP_Actors/BinObjects/BP_PickupParent.BP_PickupParent_C|GetCube _array_element_2)) (Transformation|GetWorldLocation (Variables|/Game/DEV/Taylor/BP_Actors/BinObjects/BP_PickupParent.BP_PickupParent_C|GetCube _array_element_2)) _returnvalue (Variables|/Game/DEV/Taylor/BP_Actors/BinObjects/BP_PickupParent.BP_PickupParent_C|GetObjectClass _array_element_2) (Variables|/Game/DEV/Taylor/BP_Actors/BinObjects/BP_PickupParent.BP_PickupParent_C|GetDespawnQuest _array_element_2))))
  (bind _outactors_2 (Actor|GetAllActorsOfClass "/Game/DEV/Taylor/BP_Actors/BinObjects/BP_Rubbish.BP_Rubbish_C"))
  (for _array_element_3 _outactors_2
    (bind _asbp_rubbish (Utilities|Casting|CastToBP_Rubbish _array_element_3))
    (Default|SaveRubbish _asgi_wellness_town_3 (Transformation|GetWorldLocation (Variables|/Game/DEV/Taylor/BP_Actors/BinObjects/BP_Rubbish.BP_Rubbish_C|GetDefaultSceneRoot _asbp_rubbish)) _returnvalue (Variables|/Game/DEV/Taylor/BP_Actors/BinObjects/BP_Rubbish.BP_Rubbish_C|GetCollected? _asbp_rubbish)))
  (bind _outactors_3 (Actor|GetAllActorsOfClass "/Game/DEV/Taylor/BP_Actors/NPC/BP_NPCTest.BP_NPCTest_C"))
  (for _array_element_4 _outactors_3
    (if (Utilities|Map|Contains (Variables|/Game/DEV/Taylor/GameInstance/GI_WellnessTown.GI_WellnessTown_C|GetNPCWellness _asgi_wellness_town_3) (Utilities|String|ToString(Name) (Variables|/Game/DEV/Taylor/BP_Actors/NPC/BP_NPCTest.BP_NPCTest_C|GetNPCName _array_element_4)))
      (Utilities|Map|Add (Variables|/Game/DEV/Taylor/GameInstance/GI_WellnessTown.GI_WellnessTown_C|GetNPCWellness _asgi_wellness_town_3) (Utilities|String|ToString(Name) (Variables|/Game/DEV/Taylor/BP_Actors/NPC/BP_NPCTest.BP_NPCTest_C|GetNPCName _array_element_4)) (Variables|/Game/DEV/Taylor/BP_Actors/NPC/BP_NPCTest.BP_NPCTest_C|GetWellness _array_element_4))
      (else
        (Utilities|Map|Add (Variables|/Game/DEV/Taylor/GameInstance/GI_WellnessTown.GI_WellnessTown_C|GetNPCWellness _asgi_wellness_town_3) (Utilities|String|ToString(Name) (Variables|/Game/DEV/Taylor/BP_Actors/NPC/BP_NPCTest.BP_NPCTest_C|GetNPCName _array_element_4)) (Variables|/Game/DEV/Taylor/BP_Actors/NPC/BP_NPCTest.BP_NPCTest_C|GetWellness _array_element_4)))))
  (Utilities|FlowControl|Delay 0.1)
  (bind _asbp_tp_interface_example_2 (Utilities|Casting|CastToBP_Player (Game|GetPlayerCharacter 0)))
  (bind _asgi_wellness_town_4 (Utilities|Casting|CastToGI_WellnessTown (Game|GetGameInstance)))
  (Variables|/Game/DEV/Taylor/GameInstance/GI_WellnessTown.GI_WellnessTown_C|SetPlayerCollectedItems _asgi_wellness_town_4 (Variables|/Game/DEV/Taylor/BP_CC/BP_Player.BP_Player_C|GetCollectedItems _asbp_tp_interface_example_2))
  (Variables|/Game/DEV/Taylor/GameInstance/GI_WellnessTown.GI_WellnessTown_C|SetMusic _asgi_wellness_town_4 (Variables|/Script/Engine.AudioComponent|GetSound (Variables|/Game/DEV/Taylor/GameInstance/GI_WellnessTown.GI_WellnessTown_C|GetGameMusic _asgi_wellness_town_4)))
  (Variables|/Game/DEV/Taylor/GameInstance/GI_WellnessTown.GI_WellnessTown_C|SetMusicTime _asgi_wellness_town_4 (Variables|/Game/DEV/Taylor/BP_CC/BP_Player.BP_Player_C|GetMusicTime _asbp_tp_interface_example_2))
  (Game|OpenLevel(byName) (Variables|Default|GetLevelName)))

(event EventBeginPlay
  (bind _arrow (Variables|Default|GetArrow))
  (bind _returnvalue (Transformation|GetWorldLocation _arrow))
  (bind _asgi_wellness_town (Utilities|Casting|CastToGI_WellnessTown (Game|GetGameInstance)))
  (if (Utilities|Enum|Equal(Enum) (Variables|Default|GetDoorName) (Variables|/Game/DEV/Taylor/GameInstance/GI_WellnessTown.GI_WellnessTown_C|GetSpawn _asgi_wellness_town))
    (Transformation|Teleport (Game|GetPlayerCharacter 0) _returnvalue (Math|Rotator|MakeRotator 0.0 0.0 (.yaw (Math|Rotator|FindLookatRotation (Transformation|GetWorldLocation (Variables|Default|GetDefaultSceneRoot)) _returnvalue))))))

(fn ConstructionScript
  (Transformation|SetRelativeLocation (Variables|Default|GetArrow) (Variables|Default|GetSpawnPointOffset%28Arrow%29) false false))

(fn OverlayFadein
  (CameraFades|StartCameraFade :self (Game|GetPlayerCameraManager 0) :ToAlpha (Variables|Default|GetFade_Alpha) :Duration (Variables|Default|GetFade_Duration) :bHoldWhenFinished true))