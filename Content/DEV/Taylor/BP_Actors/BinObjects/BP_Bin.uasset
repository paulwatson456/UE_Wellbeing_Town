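; Waste bin for sorting quests, coloured by Type (general, recycling, garden), that accepts matching BP_BinBag_Pickup bags either by interaction or thrown into its sphere.
; ResetBin scans the player's active quest objectives for BinName to set requirement, progress and active state.
; Each deposit advances the objective with sound, particles and widget update; meeting all ConnectedBins' requirements shows NPC approval.
; BeginPlay can give a quest based on completed-quest prerequisites.
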(event OnComponentBeginOverlap(Sphere1)
  (params (OverlappedComponent :type Primitive%20Component%20Object%20Reference) (OtherActor :type Actor%20Object%20Reference) (OtherComp :type Primitive%20Component%20Object%20Reference) (OtherBodyIndex :type Integer) (bFromSweep :type Boolean) (SweepResult :type Hit%20Result%20Structure%20%28by%20ref%29))
  ;[1 1 1] Object thrown at bin
  (bind _asbp_bin_bag_pickup (Utilities|Casting|CastToBP_BinBag_Pickup OtherActor))
  (if (Variables|Default|GetCanBinObjects)
    (if (Utilities|Enum|Equal(Enum) (Variables|/Game/DEV/Taylor/BP_Actors/BinObjects/BP_BinBag_Pickup.BP_BinBag_Pickup_C|GetType _asbp_bin_bag_pickup) (Variables|Default|GetType))
      (if (>= (Variables|Default|GetObjectsBinned) (Variables|Default|GetRequirement))
        (Development|PrintString "Finished")
        (else
          (Utilities|IsValid (Transformation|GetAttachParent (Variables|/Game/DEV/Taylor/BP_Actors/BinObjects/BP_PickupParent.BP_PickupParent_C|GetCube _asbp_bin_bag_pickup))
            (:Is%20Not%20Valid
              (CallFunction|RemoveItemfromBounds _asbp_bin_bag_pickup)
              (Actor|DestroyActor _asbp_bin_bag_pickup)
              (Development|PrintString "Not carrying")
              (Math|Integer|IncrementInt (Variables|Default|GetObjectsBinned)
                (:%20%20
                  (CallFunction|Finished)
                  (CallFunction|Particle))))))))))

(event Custom|ResetBin
  (bind _binname (Variables|Default|GetBinName))
  ;[1 1 1] Checks bin requirements - updated from quest system
  (Utilities|FlowControl|Delay 0.7)
  (bind _asbp_player (Utilities|Casting|CastToBP_Player (Game|GetPlayerCharacter 0)))
  ;;[1 1 1] Loop through all active quests
  (Variables|Default|SetLoops 0)
  (Utilities|Loop (Utilities|Array|Length (Variables|/Game/DEV/Taylor/Quests/QuestComponent.QuestComponent_C|GetCurrentQuests (Variables|/Game/DEV/Taylor/BP_CC/BP_Player.BP_Player_C|GetQuestComponent _asbp_player))) :!label _label
    (:NewParam2
      (for _array_element (.Objectives (Utilities|Struct|BreakS_StageDetails (Variables|/Game/DEV/Taylor/Quests/Quests.Quests_C|GetCurrentStageDetails (Utilities|Array|Get(acopy) (Variables|/Game/DEV/Taylor/Quests/QuestComponent.QuestComponent_C|GetCurrentQuests (Variables|/Game/DEV/Taylor/BP_CC/BP_Player.BP_Player_C|GetQuestComponent _asbp_player)) (Variables|Default|GetLoops)))))
        ;;[1 1 1] Check if quest objective "Bin" is active
        (Utilities|FlowControl|DoOnce false :!label _label_2
          (:Completed
            (if (Math|Boolean|ANDBoolean (Utilities|Enum|Equal(Enum) (.Type (Utilities|Struct|BreakS_ObjectiveDetails _array_element)) "NewEnumerator5") (Utilities|Enum|Equal(Enum) (.ObjectiveID (Utilities|Struct|BreakS_ObjectiveDetails _array_element)) _binname) (< (.Value (Utilities|Map|Find (Variables|/Game/DEV/Taylor/Quests/Quests.Quests_C|GetCurrentOpbectiveProgress (Utilities|Array|Get(acopy) (Variables|/Game/DEV/Taylor/Quests/QuestComponent.QuestComponent_C|GetCurrentQuests (Variables|/Game/DEV/Taylor/BP_CC/BP_Player.BP_Player_C|GetQuestComponent _asbp_player)) (Variables|Default|GetLoops))) _binname)) (.Quantity (Utilities|Struct|BreakS_ObjectiveDetails _array_element))))
              ;;[1 1 1] Sets the bin requirements and how many objects are in the bin then activates the bin
              (bind _output_get (Variables|Default|SetRequirement (.Quantity (Utilities|Struct|BreakS_ObjectiveDetails _array_element))))
              (bind _output_get_2 (Variables|Default|SetObjectsBinned (.Value (Utilities|Map|Find (Variables|/Game/DEV/Taylor/Quests/Quests.Quests_C|GetCurrentOpbectiveProgress (Utilities|Array|Get(acopy) (Variables|/Game/DEV/Taylor/Quests/QuestComponent.QuestComponent_C|GetCurrentQuests (Variables|/Game/DEV/Taylor/BP_CC/BP_Player.BP_Player_C|GetQuestComponent _asbp_player)) (Variables|Default|GetLoops))) _binname))))
              (CallFunction|ShowRequirements)
              (Development|PrintString (Utilities|String|Append (Utilities|String|ToString(Integer) _output_get_2) " / " (Utilities|String|ToString(Integer) _output_get))) ; Add bin requirement UI here
              (Development|SetHiddeninGame (Variables|Default|GetSphere) true true)
              (Variables|Default|SetCanBinObjects true)
              (Rendering|SetVisibility (Variables|Default|GetWidget) true false)
              (Utilities|FlowControl|Delay 0.2)
              (goto _label_2 Reset)
              (else
                ;;[1 1 1] Deactivates bin
                (Development|SetHiddeninGame (Variables|Default|GetSphere) false true)
                (Variables|Default|SetCanBinObjects false)
                (Rendering|SetVisibility (Variables|Default|GetWidget) false false)
                (goto _label_2 Reset))))))
      (Math|Integer|IncrementInt (Variables|Default|GetLoops)
        (:%20%20
          (goto _label))))))

(event Custom|Particle
  (bind _niagara (Variables|Default|GetNiagara))
  ;[1 1 1] Bin particles
  (Components|Activation|SetActive _niagara true false)
  (Utilities|FlowControl|Delay 0.5)
  (Components|Activation|SetActive _niagara false false))

(event Custom|Dialogue
  ;[1 1 1] Bin dialogue
  (bind _asbp_player (Utilities|Casting|CastToBP_Player (Game|GetPlayerCharacter 0)))
  (bind _aswi_dialogue (Utilities|Casting|CastToWI_Dialogue (UserInterface|GetWidget (Variables|/Game/DEV/Taylor/BP_CC/BP_Player.BP_Player_C|GetDialogue _asbp_player))))
  (Default|SetThoughtBubble _aswi_dialogue)
  (if (Variables|/Game/DEV/Taylor/BP_CC/BP_Player.BP_Player_C|GetCarryingObject _asbp_player)
    (if (and (Variables|Default|GetCanBinObjects) (== (Variables|/Game/DEV/Taylor/BP_Actors/BinObjects/BP_PickupParent.BP_PickupParent_C|GetObjectClass (Variables|/Game/DEV/Taylor/BP_CC/BP_Player.BP_Player_C|GetBag _asbp_player)) "/Game/DEV/Taylor/BP_Actors/BinObjects/BP_BinBag_Pickup.BP_BinBag_Pickup_C"))
      (bind _asbp_bin_bag_pickup (Utilities|Casting|CastToBP_BinBag_Pickup (Variables|/Game/DEV/Taylor/BP_CC/BP_Player.BP_Player_C|GetBag _asbp_player))
        (:then
          (if (Utilities|Enum|Equal(Enum) (Variables|/Game/DEV/Taylor/BP_Actors/BinObjects/BP_BinBag_Pickup.BP_BinBag_Pickup_C|GetType _asbp_bin_bag_pickup) (Variables|Default|GetType))
            (Default|SetDialogueBubble _aswi_dialogue)
            (else
              (Default|PlayerDialogue _asbp_player "I shouldnt bin this here." true :!label _label)
              (CallFunction|ShowRequirements))))
        (:CastFailed
          (goto _label)))
      (else
        (goto _label)))
    (else
      (Default|PlayerDialogue _asbp_player "I have nothing to bin." true)
      (CallFunction|ShowRequirements))))

(event Custom|Deactivate
  (bind _binname (Variables|Default|GetBinName))
  ;[1 1 1] Checks bin requirements - updated from quest system
  ;;[1 1 1] Deactivates bin
  (Development|SetHiddeninGame (Variables|Default|GetSphere) false true)
  (Variables|Default|SetCanBinObjects false)
  (Rendering|SetVisibility (Variables|Default|GetWidget) false false)
  ;;[1 1 1] Check if quest objective "Bin" is active
  (Utilities|FlowControl|DoOnce false) ; enters at Reset
)

(event EventBeginPlay
  (bind _donottriggerifquestcomplete (Variables|Default|GetDoNotTriggerifQuestComplete))
  (Utilities|FlowControl|Delay 0.19)
  (bind _asgi_wellness_town (Utilities|Casting|CastToGI_WellnessTown (Game|GetGameInstance)))
  (if (Math|Boolean|ANDBoolean (Utilities|Array|ContainsItem (Variables|/Game/DEV/Taylor/GameInstance/GI_WellnessTown.GI_WellnessTown_C|GetCompletedQuests _asgi_wellness_town) (Variables|Default|GetQuestRequirement)) (!= (.rowname (Variables|/Game/DEV/Taylor/Quests/QuestGiverComponent.QuestGiverComponent_C|GetQuestData (Variables|Default|GetQuestGiverComponent))) "") (or (not (Utilities|Array|ContainsItem (Variables|/Game/DEV/Taylor/GameInstance/GI_WellnessTown.GI_WellnessTown_C|GetCompletedQuests _asgi_wellness_town) _donottriggerifquestcomplete)) (== _donottriggerifquestcomplete "None")))
    (Default|GiveQuest (Variables|Default|GetQuestGiverComponent))))

(event EventShowPrompt
  ;[1 1 1] Interaction
  ;;[1 1 1] Interaction prompt
  (bind _asbp_player (Utilities|Casting|CastToBP_Player (Game|GetPlayerCharacter 0)))
  (bind _asbp_interact_prompt (Utilities|Casting|CastToBP_InteractPrompt (Variables|/Script/Engine.ChildActorComponent|GetChildActor (Variables|Default|GetBP_InteractPrompt))))
  (Default|ShowPrompt _asbp_interact_prompt))

(event EventGeneralInteract
  ;[1 1 1] Interaction
  ;;[1 1 1] Interact
  (bind _asbp_player (Utilities|Casting|CastToBP_Player (Game|GetPlayerCharacter 0)))
  (bind _asbp_bin_bag_pickup (Utilities|Casting|CastToBP_BinBag_Pickup (Variables|/Game/DEV/Taylor/BP_CC/BP_Player.BP_Player_C|GetBag _asbp_player))
    (:then
      _)
    (:CastFailed
      _))
  (if (Math|Boolean|ANDBoolean (Variables|Default|GetCanBinObjects) (Variables|/Game/DEV/Taylor/BP_CC/BP_Player.BP_Player_C|GetCarryingObject _asbp_player) (not (>= (Variables|Default|GetObjectsBinned) (Variables|Default|GetRequirement))))
    (if (== (Variables|/Game/DEV/Taylor/BP_Actors/BinObjects/BP_PickupParent.BP_PickupParent_C|GetObjectClass (Variables|/Game/DEV/Taylor/BP_CC/BP_Player.BP_Player_C|GetBag _asbp_player)) "/Game/DEV/Taylor/BP_Actors/BinObjects/BP_BinBag_Pickup.BP_BinBag_Pickup_C")
      (if (Utilities|Enum|Equal(Enum) (Variables|/Game/DEV/Taylor/BP_Actors/BinObjects/BP_BinBag_Pickup.BP_BinBag_Pickup_C|GetType _asbp_bin_bag_pickup) (Variables|Default|GetType))
        (Variables|/Game/DEV/Taylor/BP_CC/BP_Player.BP_Player_C|SetCarryingObject _asbp_player false)
        (CallFunction|RemoveItemfromBounds (Variables|/Game/DEV/Taylor/BP_CC/BP_Player.BP_Player_C|GetBag _asbp_player))
        (Actor|DestroyActor (Variables|/Game/DEV/Taylor/BP_CC/BP_Player.BP_Player_C|GetBag _asbp_player))
        (Variables|/Game/DEV/Taylor/BP_CC/BP_Player.BP_Player_C|SetBag _asbp_player 0)
        (Widget|RemovefromParent (Variables|/Game/DEV/Taylor/BP_CC/BP_Player.BP_Player_C|GetPromptWidget _asbp_player))
        (Development|PrintString "Carrying")
        (Math|Integer|IncrementInt (Variables|Default|GetObjectsBinned)
          (:%20%20
            (CallFunction|Finished)
            (CallFunction|Particle)))
        (else
          (CallFunction|Dialogue :!label _label)))
      (else
        (goto _label)))
    (else
      (goto _label))))

(fn ConstructionScript
  (Development|SetHiddeninGame (Variables|Default|GetSphere) true true)
  (switch Utilities|FlowControl|Switch|SwitchonE_BinType (Variables|Default|GetType)
    (:NewEnumerator0
      (Rendering|Material|SetMaterial (Variables|Default|GetCube) 0 "/Game/DEV/Taylor/Materials/M_Base.M_Base"))
    (:NewEnumerator1
      (Rendering|Material|SetMaterial (Variables|Default|GetCube) 0 "/Game/DEV/Taylor/Materials/M_Blue.M_Blue"))
    (:NewEnumerator2
      (Rendering|Material|SetMaterial (Variables|Default|GetCube) 0 "/Game/DEV/Taylor/Materials/M_Green1.M_Green1"))))

(fn Finished
  (bind _asbp_player (Utilities|Casting|CastToBP_Player (Game|GetPlayerCharacter 0)))
  (Default|ObjectiveProgress _asbp_player (Variables|Default|GetBinName))
  (Audio|PlaySoundatLocation "/Game/DEV/Taylor/Sound/BinObjects.BinObjects" (Transformation|GetWorldLocation (Variables|Default|GetCube)) "0, 0, 0" 1.0 0.8 0.0 0 0 0 0)
  (if (>= (Variables|Default|GetObjectsBinned) (Variables|Default|GetRequirement))
    (Development|SetHiddeninGame (Variables|Default|GetSphere) false true)
    (CallFunction|Deactivate)
    (CallFunction|NPCApproval))
  (CallFunction|ShowRequirements))

(fn ShowRequirements
  (bind _asbin_requirements (Utilities|Casting|CastToBinRequirements (UserInterface|GetWidget (Variables|Default|GetWidget1))))
  (Default|ShowProgress _asbin_requirements (Variables|Default|GetObjectsBinned) (Variables|Default|GetRequirement)))

(fn RemoveItemfromBounds
  (params (Item :type BP%20Pickup%20Parent%20Object%20Reference))
  (bind _bounds (Variables|Default|GetBounds))
  (Utilities|IsValid _bounds
    (:Is%20Valid
      (Default|RemoveItem _bounds Item))))

(fn NPCApproval
  (LocalVariables|SetRequirementMet true)
  (for _array_element (Variables|Default|GetConnectedBins)
    (if (not (>= (Variables|BP_Bin_C|GetObjectsBinned _array_element) (Variables|BP_Bin_C|GetRequirement _array_element)))
      (LocalVariables|SetRequirementMet false)))
  (if (LocalVariables|GetRequirementMet)
    (for _array_element_2 (Variables|Default|GetNPCForApproval)
      ;[1 1 1] Shows face above NPC's head
      (bind _aswi_faces (Utilities|Casting|CastToWI_Faces (UserInterface|GetWidget (Variables|/Game/DEV/Taylor/BP_Actors/NPC/BP_NPCTest.BP_NPCTest_C|GetDialogueApproval _array_element_2))))
      (Class|Image|SetOpacity (Variables|/Game/DEV/Taylor/Widgets/WI_Faces.WI_Faces_C|GetImage_0 _aswi_faces) 1.0)
      (Class|Image|SetBrush (Variables|/Game/DEV/Taylor/Widgets/WI_Faces.WI_Faces_C|GetImage_0 _aswi_faces) (Utilities|Struct|MakeSlateBrush "Image" "NoTile" "NoMirror" "(X=32.000000,Y=32.000000)" "(Left=0.000000,Top=0.000000,Right=0.000000,Bottom=0.000000)" "(SpecifiedColor=(R=1.000000,G=1.000000,B=1.000000,A=1.000000),ColorUseRule=UseColor_Specified)" "(CornerRadii=(X=0.000000,Y=0.000000,Z=0.000000,W=0.000000),Color=(SpecifiedColor=(R=0.000000,G=0.000000,B=0.000000,A=0.000000),ColorUseRule=UseColor_Specified),Width=0.000000,RoundingType=HalfHeightRadius,bUseBrushTransparency=False)" "/Game/DEV/Taylor/Widgets/Images/icons8-happy-100__1_.icons8-happy-100__1_"))
      (Audio|SpawnSoundAttached "/Game/DEV/Taylor/Sound/DialogueResult.DialogueResult" (Variables|/Script/Engine.Actor|GetRootComponent _array_element_2) "None" "0, 0, 0" "0, 0, 0" "KeepRelativeOffset" false 1.0 1.35 0.0 "/Game/DEV/Taylor/Sound/Attenuation/Atten_Short.Atten_Short" 0)
      (Default|Finished _aswi_faces 2)
      ;[1 1 1] Uses Pickup UI to display NPC approval
      (bind _asbp_player (Utilities|Casting|CastToBP_Player (Game|GetPlayerCharacter 0)))
      (Default|PickUp1 _asbp_player "/Game/DEV/Taylor/Widgets/Images/icons8-happy-100__1_.icons8-happy-100__1_" (Variables|/Game/DEV/Taylor/BP_Actors/NPC/BP_NPCTest.BP_NPCTest_C|GetNPCName _array_element_2) ": Approved " false))))