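; Parent pickup actor that the player can carry and throw, with an interact prompt shown only when hands are free.
; On BeginPlay and quest updates, it destroys itself if a quest's stage matches DespawnQuest.
; Tick controls thrown rotation, tilting curved throws by vertical velocity or settling normal ones.
; Hits can restore player-channel blocking, freeze quest items and play speed-scaled sounds, while TeleportItem relocates it after a delay.
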(event OnComponentHit(Cube)
  (params (HitComponent :type Primitive%20Component%20Object%20Reference) (OtherActor :type Actor%20Object%20Reference) (OtherComp :type Primitive%20Component%20Object%20Reference) (NormalImpulse :type Vector :default "0, 0, 0") (Hit :type Hit%20Result%20Structure%20%28by%20ref%29))
  (bind _cube (Variables|Default|GetCube))
  (bind _returnvalue (Transformation|GetComponentVelocity _cube))
  (bind _returnvalue_2 (Math|Vector|VectorLength _returnvalue))
  ;[1 1 1] Triggered when item hits something after being thrown
  ;;[1 1 1] Checks if item should collide with the player - Box pickup
  (if (Variables|Default|GetBlockPlayerCol?)
    (if (Physics|IsSimulatingPhysics (Variables|Default|GetCube) "None")
      (Collision|SetCollisionResponsetoChannel (Variables|Default|GetCube) "ECC_GameTraceChannel2" "ECR_Block")
      ;;[1 1 1] Checks if item should bounce
      (if (Variables|Default|GetQuestItem?) :!label _label
        (Physics|SetSimulatePhysics (Variables|Default|GetCube) false))
      ;;[1 1 1] If item has enough velocity it plays a sound when bouncing
      (if (> _returnvalue_2 2e+02)
        (Utilities|FlowControl|DoOnce false :!label _label_2
          (:Completed
            (Audio|PlaySoundatLocation (Variables|Default|GetSound) (Transformation|GetWorldLocation _cube) "0, 0, 0" (/ _returnvalue_2 1.5e+03) 1.0 0.0 0 0 0 0)
            (Utilities|FlowControl|Delay 0.1)
            (goto _label_2 Reset)))))
    (else
      (goto _label))))

(event Custom|QuestUpdate
  ;[1 1 1] Despawns pickup if the quest tells it to
  (Utilities|FlowControl|Delay 0.4)
  (bind _outactors (Actor|GetAllActorsOfClass "/Game/DEV/Taylor/Quests/Quests.Quests_C"))
  (for _array_element _outactors
    (if (Utilities|Enum|Equal(Enum) (.stagename (Variables|/Game/DEV/Taylor/Quests/Quests.Quests_C|GetCurrentStageDetails _array_element)) (Variables|Default|GetDespawnQuest))
      (Actor|DestroyActor))))

(event Custom|AlignPickupRotationWithPlayer
  ;[1 1 1] Interactions
  ;;[1 1 1] Interact - Pickup item
  (Utilities|FlowControl|DoOnce false
    (:Completed
      (Variables|Default|SetRotation (Transformation|GetWorldRotation (Variables|/Script/Engine.Character|GetCapsuleComponent (Game|GetPlayerCharacter 0)))))))

(event Custom|UniqueDrop)

(event Custom|UniquePickup)

(event Custom|TeleportItem
  (params (Delay :type Float%20%28double-precision%29) (Location :type Vector))
  (bind _cube (Variables|Default|GetCube))
  (Utilities|FlowControl|DoOnce false :!label _label
    (:Completed
      (Utilities|FlowControl|Delay Delay)
      (Transformation|SetWorldLocation _cube Location false true)
      (Physics|SetPhysicsLinearVelocity _cube "0, 0, 0" false "None")
      (Audio|PlaySoundatLocation "/Engine/VREditor/Sounds/UI/Drop_Item_From_ContentBrowser.Drop_Item_From_ContentBrowser" Location "0, 0, 0" 1.0 1.0 0.0 0 0 0 0)
      (Physics|SetSimulatePhysics (Variables|Default|GetCube) true)
      (goto _label Reset))))

(event EventBeginPlay
  ;[1 1 1] Despawns pickup if the quest tells it to
  (Variables|Default|SetObjectClass (Utilities|GetClass self))
  (Utilities|FlowControl|Delay 0.4)
  (bind _outactors (Actor|GetAllActorsOfClass "/Game/DEV/Taylor/Quests/Quests.Quests_C"))
  (for _array_element _outactors
    (if (Utilities|Enum|Equal(Enum) (.stagename (Variables|/Game/DEV/Taylor/Quests/Quests.Quests_C|GetCurrentStageDetails _array_element)) (Variables|Default|GetDespawnQuest))
      (Actor|DestroyActor))))

(event EventTick
  (params (DeltaSeconds :type Float%20%28single-precision%29))
  (bind _rotation (Variables|Default|GetRotation))
  (bind _cube (Variables|Default|GetCube))
  ;[1 1 1] Throwing
  (if (Physics|IsSimulatingPhysics (Variables|Default|GetCube) "None")
    (if (Variables|Default|GetCurve?)
      ;;[1 1 1] Throw with curve
      (Utilities|FlowControl|Sequence
        (:then_0
          (CallFunction|AlignPickupRotationwithPlayer))
        (:then_1
          (Transformation|SetRelativeRotation _cube (Math|Rotator|MakeRotator (+ (/ (.z (Transformation|GetComponentVelocity _cube)) 2e+01) 9e+01) (.pitch _rotation) (+ (.yaw _rotation) 9e+01)) false false)))
      (else
        ;;[1 1 1] Normal throw
        (if (Variables|Default|GetSetRot?)
          (Transformation|SetWorldRotation (Variables|Default|GetCube) (Variables|Default|GetRotation) false false)
          (Utilities|FlowControl|Sequence
            (:then_0
              (CallFunction|AlignPickupRotationwithPlayer))
            (:then_1
              (Utilities|FlowControl|Delay 0.2)
              (if (Utilities|Operators|EqualEqual :A (Transformation|GetComponentVelocity (Variables|Default|GetCube)) :ErrorTolerance 5.0)
                (Physics|SetSimulatePhysics (Variables|Default|GetCube) false)
                (CallFunction|AlignPickupRotationwithPlayer)))))))))

(event EventGeneralInteract
  ;[1 1 1] Interactions
  ;;[1 1 1] Interact - Pickup item
  (bind _asbp_player (Utilities|Casting|CastToBP_Player (Game|GetPlayerCharacter 0)))
  (if (not (Variables|/Game/DEV/Taylor/BP_CC/BP_Player.BP_Player_C|GetCarryingObject _asbp_player))
    (Default|BinBagPickup _asbp_player self)
    (Utilities|FlowControl|DoOnce false) ; enters at Reset
  ))

(event EventShowPrompt
  ;[1 1 1] Interactions
  ;;[1 1 1] Interaction prompt
  (bind _asbp_player (Utilities|Casting|CastToBP_Player (Game|GetPlayerCharacter 0)))
  (if (not (Variables|/Game/DEV/Taylor/BP_CC/BP_Player.BP_Player_C|GetCarryingObject _asbp_player))
    (bind _asbp_interact_prompt (Utilities|Casting|CastToBP_InteractPrompt (Variables|/Script/Engine.ChildActorComponent|GetChildActor (Variables|Default|GetBP_InteractPrompt))))
    (Default|ShowPrompt _asbp_interact_prompt)))

(fn ConstructionScript)