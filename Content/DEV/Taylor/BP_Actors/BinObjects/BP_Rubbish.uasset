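; Interactable rubbish actor that the player collects as a bin bag during matching quest objectives.
; On delayed BeginPlay or ResetRubbish, it scans Quests actors' current objectives by type and ObjectiveID, toggling visibility, collision and Active, with debug prints.
; While active and the player's hands are free, it shows a prompt; interacting spawns a bag for the player, registers it with matching Col_ItemBounds and hides the rubbish.
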(event Custom|ResetRubbish
  (bind _outactors (Actor|GetAllActorsOfClass "/Game/DEV/Taylor/Quests/Quests.Quests_C"))
  (Variables|Default|SetLoops 0)
  (Utilities|Loop (Utilities|Array|Length _outactors) :!label _label
    (:NewParam2
      (for _array_element (.objectives (Variables|/Game/DEV/Taylor/Quests/Quests.Quests_C|GetCurrentStageDetails (Utilities|Array|Get(acopy) _outactors (Variables|Default|GetLoops))))
        (Utilities|FlowControl|DoOnce false :!label _label_2
          (:Completed
            (if (Math|Boolean|ANDBoolean (Utilities|Enum|Equal(Enum) (.Type (Utilities|Struct|BreakS_ObjectiveDetails _array_element)) "NewEnumerator5") (Utilities|Enum|Equal(Enum) (.ObjectiveID (Utilities|Struct|BreakS_ObjectiveDetails _array_element)) (Variables|Default|GetObjectiveID)) (not (Variables|Default|GetCollected?)))
              (Development|PrintString "BinQuest")
              (Rendering|SetActorHiddenInGame false)
              (Collision|SetCollisionObjectType (Variables|Default|GetCube) "ECC_WorldStatic")
              (Variables|Default|SetActive true)
              (Utilities|FlowControl|Delay 0.2)
              (goto _label_2 Reset)
              (else
                (Development|PrintString "NotBinQuest")
                (Rendering|SetActorHiddenInGame true)
                (Collision|SetCollisionObjectType (Variables|Default|GetCube) "ECC_WorldDynamic")
                (Variables|Default|SetActive false)
                (goto _label_2 Reset))))))
      (Math|Integer|IncrementInt (Variables|Default|GetLoops)
        (:%20%20
          (goto _label))))))

(event EventBeginPlay
  (Utilities|FlowControl|Delay 0.4)
  (bind _outactors (Actor|GetAllActorsOfClass "/Game/DEV/Taylor/Quests/Quests.Quests_C"))
  (Variables|Default|SetLoops 0)
  (Utilities|Loop (Utilities|Array|Length _outactors) :!label _label
    (:NewParam2
      (for _array_element (.objectives (Variables|/Game/DEV/Taylor/Quests/Quests.Quests_C|GetCurrentStageDetails (Utilities|Array|Get(acopy) _outactors (Variables|Default|GetLoops))))
        (Utilities|FlowControl|DoOnce false :!label _label_2
          (:Completed
            (if (Math|Boolean|ANDBoolean (Utilities|Enum|Equal(Enum) (.Type (Utilities|Struct|BreakS_ObjectiveDetails _array_element)) "NewEnumerator5") (Utilities|Enum|Equal(Enum) (.ObjectiveID (Utilities|Struct|BreakS_ObjectiveDetails _array_element)) (Variables|Default|GetObjectiveID)) (not (Variables|Default|GetCollected?)))
              (Development|PrintString "BinQuest")
              (Rendering|SetActorHiddenInGame false)
              (Collision|SetCollisionObjectType (Variables|Default|GetCube) "ECC_WorldStatic")
              (Variables|Default|SetActive true)
              (Utilities|FlowControl|Delay 0.2)
              (goto _label_2 Reset)
              (else
                (Development|PrintString "NotBinQuest")
                (Rendering|SetActorHiddenInGame true)
                (Collision|SetCollisionObjectType (Variables|Default|GetCube) "ECC_WorldDynamic")
                (Variables|Default|SetActive false)
                (goto _label_2 Reset))))))
      (Math|Integer|IncrementInt (Variables|Default|GetLoops)
        (:%20%20
          (goto _label))))))

(event EventGeneralInteract
  (if (Variables|Default|GetActive)
    (bind _asbp_player (Utilities|Casting|CastToBP_Player (Game|GetPlayerCharacter 0)))
    (if (not (Variables|/Game/DEV/Taylor/BP_CC/BP_Player.BP_Player_C|GetCarryingObject _asbp_player))
      (bind _returnvalue (Game|SpawnActorfromClass "/Game/DEV/Taylor/BP_Actors/BinObjects/BP_BinBag_Pickup.BP_BinBag_Pickup_C" (Math|Transform|MakeTransform "0, 0, 0" "0, 0, 0" "1.000000,1.000000,1.000000") "Undefined" "MultiplyWithRoot" 0 0))
      (Default|BinBagPickup _asbp_player _returnvalue)
      (CallFunction|AddtoBounds _returnvalue)
      (Variables|Default|SetCollected? true)
      (Rendering|SetVisibility (Variables|Default|GetDefaultSceneRoot) false true)
      (Collision|SetCollisionObjectType (Variables|Default|GetSphere) "ECC_WorldDynamic"))))

(event EventShowPrompt
  (if (Variables|Default|GetActive)
    (bind _asbp_player (Utilities|Casting|CastToBP_Player (Game|GetPlayerCharacter 0)))
    (if (not (Variables|/Game/DEV/Taylor/BP_CC/BP_Player.BP_Player_C|GetCarryingObject _asbp_player))
      (bind _asbp_interact_prompt (Utilities|Casting|CastToBP_InteractPrompt (Variables|/Script/Engine.ChildActorComponent|GetChildActor (Variables|Default|GetBP_InteractPrompt))))
      (Default|ShowPrompt _asbp_interact_prompt))))

(fn ConstructionScript)

(fn IsActive
  (params (Collected :type Boolean))
  (bind _output_get (Variables|Default|SetCollected? Collected))
  (if _output_get
    (Rendering|SetVisibility (Variables|Default|GetDefaultSceneRoot) false true)
    (Collision|SetCollisionObjectType (Variables|Default|GetSphere) "ECC_WorldDynamic")
    (Variables|Default|SetActive false)))

(fn AddtoBounds
  (params (Item :type BP%20Pickup%20Parent%20Object%20Reference))
  (if (not (Utilities|Array|IsEmpty (Variables|Default|GetObjectBounds)))
    (bind _outactors (Actor|GetAllActorsOfClass "/Game/DEV/Taylor/BP_Actors/BinObjects/Col_ItemBounds.Col_ItemBounds_C"))
    (for _array_element _outactors
      (if (Utilities|Enum|Equal(Enum) (Variables|/Game/DEV/Taylor/BP_Actors/BinObjects/Col_ItemBounds.Col_ItemBounds_C|GetCollisionID _array_element) (Variables|Default|GetObjectBounds))
        (Utilities|Map|Add (Variables|/Game/DEV/Taylor/BP_Actors/BinObjects/Col_ItemBounds.Col_ItemBounds_C|GetItems _array_element) Item (Variables|Default|GetBounds%20Dialogue))))))