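; BP_Log_Container is an objective container that collects up to three BP_Log_Pickup actors overlapping its Box.
; Each deposit destroys the pickup, reveals the next log component and reports objective progress to BP_Player by Name, provided that player cast succeeds.
; The third log makes a valid linked NPC show new dialogue, optionally restoring its previous dialogue after a delay.
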(event OnComponentBeginOverlap(Box)
  (params (OverlappedComponent :type Primitive%20Component%20Object%20Reference) (OtherActor :type Actor%20Object%20Reference) (OtherComp :type Primitive%20Component%20Object%20Reference) (OtherBodyIndex :type Integer) (bFromSweep :type Boolean) (SweepResult :type Hit%20Result%20Structure%20%28by%20ref%29))
  (bind _logs (Variables|Default|GetLogs))
  (bind _npc (Variables|Default|GetNPC))
  (bind _asbp_log_pickup (Utilities|Casting|CastToBP_Log_Pickup OtherActor))
  (if (< (Variables|Default|GetLogs) 3)
    (Math|Integer|IncrementInt (Variables|Default|GetLogs)
      (:%20%20
        (Actor|DestroyActor _asbp_log_pickup)
        (bind _asbp_tp_interface_example (Utilities|Casting|CastToBP_Player (Game|GetPlayerCharacter 0)))
        (Default|ObjectiveProgress _asbp_tp_interface_example (Variables|Default|GetName))
        (if (== _logs 1)
          (Rendering|SetVisibility (Variables|Default|GetLog1) true false)
          (elif (== _logs 2)
            (Rendering|SetVisibility (Variables|Default|GetLog2) true false)
            (else
              (Rendering|SetVisibility (Variables|Default|GetLog3) true false)
              (Utilities|IsValid (Variables|Default|GetNPC)
                (:Is%20Valid
                  (Variables|Default|SetNPCDialogue (Variables|/Game/DEV/Taylor/BP_Actors/NPC/BP_NPCTest.BP_NPCTest_C|GetDialogue _npc))
                  (Variables|/Game/DEV/Taylor/BP_Actors/NPC/BP_NPCTest.BP_NPCTest_C|SetDialogue _npc (Variables|Default|GetNewDialogue))
                  (Default|ShowDialogue _npc)
                  (if (Variables|Default|GetSetDialogueback)
                    (Utilities|FlowControl|Delay 5.0)
                    (Variables|/Game/DEV/Taylor/BP_Actors/NPC/BP_NPCTest.BP_NPCTest_C|SetDialogue _npc (Variables|Default|GetNPCDialogue))))))))))))

(event EventBeginPlay)

(event Collision|EventActorBeginOverlap
  (params (OtherActor :type Actor%20Object%20Reference)))

(event EventTick
  (params (DeltaSeconds :type Float%20%28single-precision%29)))

(fn ConstructionScript)