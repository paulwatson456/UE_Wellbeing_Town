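; Level-transition door trigger that moves the player between maps and places them at the matching door on arrival.
; When BP_Player overlaps the box, it fades the camera, waits briefly, stores DoorName in GI_WellnessTown's Spawn and opens LevelName.
; On BeginPlay, the instance whose DoorName matches Spawn teleports the player character to its Arrow's location.
; An older DoorPosition save-game version of this handoff remains unconnected in the graph.
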(event OnComponentBeginOverlap(Box)
  (params (OverlappedComponent :type Primitive%20Component%20Object%20Reference) (OtherActor :type Actor%20Object%20Reference) (OtherComp :type Primitive%20Component%20Object%20Reference) (OtherBodyIndex :type Integer) (bFromSweep :type Boolean) (SweepResult :type Hit%20Result%20Structure%20%28by%20ref%29))
  (Utilities|Casting|CastToBP_Player OtherActor)
  (CallFunction|SetSpawnPos))

(event Custom|SetSpawnPos
  (CallFunction|OverlayFadein)
  (Utilities|FlowControl|Delay 0.75)
  (bind _asgi_wellness_town (Utilities|Casting|CastToGI_WellnessTown (Game|GetGameInstance)))
  (Variables|/Game/DEV/Taylor/GameInstance/GI_WellnessTown.GI_WellnessTown_C|SetSpawn _asgi_wellness_town (Variables|Default|GetDoorName))
  (Game|OpenLevel(byName) (Variables|Default|GetLevelName)))

(event EventBeginPlay
  (bind _asgi_wellness_town (Utilities|Casting|CastToGI_WellnessTown (Game|GetGameInstance)))
  (if (Utilities|Enum|Equal(Enum) (Variables|Default|GetDoorName) (Variables|/Game/DEV/Taylor/GameInstance/GI_WellnessTown.GI_WellnessTown_C|GetSpawn _asgi_wellness_town))
    (Transformation|Teleport (Game|GetPlayerCharacter 0) (Transformation|GetWorldLocation (Variables|Default|GetArrow)) "0, 0, 0")))

(event Collision|EventActorBeginOverlap
  (params (OtherActor :type Actor%20Object%20Reference)))

(event EventTick
  (params (DeltaSeconds :type Float%20%28single-precision%29)))

(fn ConstructionScript)

(fn OverlayFadein
  (CameraFades|StartCameraFade :self (Game|GetPlayerCameraManager 0) :ToAlpha 1.5 :Duration 0.5 :bHoldWhenFinished true))