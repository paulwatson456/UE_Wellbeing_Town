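; Inspectable quest item that appears only if its name is in the player's quest rewards, otherwise destroying itself shortly after BeginPlay.
; Interacting through the child-actor prompt blends the view to the item, hides the player and moves input to the item until F closes it.
; A widget banner shows the name and description looked up from the player.
; The construction script builds its look from configurable meshes, transforms and materials.
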(event Custom|Interact
  (bind _returnvalue (Game|GetPlayerController 0))
  (bind _asbp_interact_prompt (Utilities|Casting|CastToBP_InteractPrompt (Variables|/Script/Engine.ChildActorComponent|GetChildActor (Variables|Default|GetBP_InteractPrompt))))
  (Variables|/Game/DEV/Taylor/BP_Actors/BP_InteractPrompt.BP_InteractPrompt_C|SetCanInteract? _asbp_interact_prompt false)
  (Game|Player|SetViewTargetwithBlend (Game|GetPlayerController 0) self 0.0 "VTBlend_Linear" 0.0 false)
  (Input|EnableInput _returnvalue)
  (Input|DisableInput (Game|GetPlayerCharacter 0) _returnvalue)
  (bind _aswi_item_collected_banner (Utilities|Casting|CastToWI_ItemCollectedBanner (UserInterface|GetWidget (Variables|Default|GetDescription))))
  (Default|Interacted _aswi_item_collected_banner)
  (Rendering|SetActorHiddenInGame (Game|GetPlayerCharacter 0) true))

(event EventBeginPlay
  (Utilities|FlowControl|Delay 0.2)
  (bind _asbp_tp_interface_example (Utilities|Casting|CastToBP_Player (Game|GetPlayerCharacter 0)))
  (if (Utilities|Array|ContainsItem (Variables|/Game/DEV/Taylor/BP_CC/BP_Player.BP_Player_C|GetQuestRewards _asbp_tp_interface_example) (Variables|Default|GetName))
    (bind _aswi_item_collected_banner (Utilities|Casting|CastToWI_ItemCollectedBanner (UserInterface|GetWidget (Variables|Default|GetDescription))))
    (Variables|/Game/DEV/Taylor/Widgets/WI_ItemCollectedBanner.WI_ItemCollectedBanner_C|SetName _aswi_item_collected_banner (Variables|Default|GetName))
    (Variables|/Script/UMG.MultiLineEditableText|SetText (Variables|/Game/DEV/Taylor/Widgets/WI_ItemCollectedBanner.WI_ItemCollectedBanner_C|GetMultiLineEditableText_0 _aswi_item_collected_banner) (Utilities|Text|ToText(Name) (.Value (Utilities|Map|Find (Variables|/Game/DEV/Taylor/BP_CC/BP_Player.BP_Player_C|GetItemDescriptions _asbp_tp_interface_example) (Variables|Default|GetName)))))
    (else
      (Actor|DestroyActor))))

(event EventShowPrompt
  ;[0.05127 0.05127 0.05127] ButtonPrompt
  (bind _asbp_interact_prompt (Utilities|Casting|CastToBP_InteractPrompt (Variables|/Script/Engine.ChildActorComponent|GetChildActor (Variables|Default|GetBP_InteractPrompt))))
  (Default|ShowPrompt _asbp_interact_prompt))

(event EventGeneralInteract
  ;[0.05127 0.05127 0.05127] Primary Interaction
  (bind _asbp_interact_prompt (Utilities|Casting|CastToBP_InteractPrompt (Variables|/Script/Engine.ChildActorComponent|GetChildActor (Variables|Default|GetBP_InteractPrompt))))
  (if (Variables|/Game/DEV/Taylor/BP_Actors/BP_InteractPrompt.BP_InteractPrompt_C|GetCanInteract? _asbp_interact_prompt)
    (CallFunction|Interact)))

(event Input|KeyboardEvents|F
  (params (Key :type Key%20Structure))
  (bind _returnvalue (Game|GetPlayerController 0))
  (:Pressed
    (bind _asbp_interact_prompt (Utilities|Casting|CastToBP_InteractPrompt (Variables|/Script/Engine.ChildActorComponent|GetChildActor (Variables|Default|GetBP_InteractPrompt))))
    (Variables|/Game/DEV/Taylor/BP_Actors/BP_InteractPrompt.BP_InteractPrompt_C|SetCanInteract? _asbp_interact_prompt true)
    (Game|Player|SetViewTargetwithBlend (Game|GetPlayerController 0) (Game|GetPlayerCharacter 0) 0.0 "VTBlend_Linear" 0.0 false)
    (Input|EnableInput (Game|GetPlayerCharacter 0) _returnvalue)
    (Input|DisableInput _returnvalue)
    (bind _aswi_item_collected_banner (Utilities|Casting|CastToWI_ItemCollectedBanner (UserInterface|GetWidget (Variables|Default|GetDescription))))
    (Default|Closed _aswi_item_collected_banner)
    (Rendering|SetActorHiddenInGame (Game|GetPlayerCharacter 0) false)))

(fn ConstructionScript
  (bind _cube (Variables|Default|GetCube))
  (bind _additionalmesh (Variables|Default|GetAdditionalMesh))
  (Transformation|SetRelativeTransform _cube (Variables|Default|GetTransform) false false)
  (Components|StaticMesh|SetStaticMesh _cube (Variables|Default|GetMesh))
  (for (_array_element _array_index) (Variables|Default|GetMaterial)
    (Rendering|Material|SetMaterial _cube _array_index _array_element))
  (bind _keys (Utilities|Map|Keys _additionalmesh))
  (for (_array_element_2 _array_index_2) _keys
    (bind _values (Utilities|Map|Values _additionalmesh))
    (bind _returnvalue (AddComponent|AddStaticMeshComponent false))
    (Components|StaticMesh|SetStaticMesh _returnvalue _array_element_2)
    (Transformation|SetRelativeTransform _returnvalue (Utilities|Array|Get(acopy) _values _array_index_2) false false)
    (Rendering|Material|SetMaterial _returnvalue 0 (Utilities|Array|Get(acopy) (Variables|Default|GetAdditionalMaterials) _array_index_2))))