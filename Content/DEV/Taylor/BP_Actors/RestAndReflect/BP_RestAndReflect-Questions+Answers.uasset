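; Rest and Reflect actor that supplies the question and answer data for the game's reflection scenes.
; On BeginPlay it uses the reflection scene number saved in GI_WellnessTown to index the data table's row names, then caches that row for GetDataForReflectionQuestions to return.
; The index lookup is a stopgap for querying the objective system; an unconnected quest-progress experiment remains in the graph.
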(event EventBeginPlay
  ;[1 1 1] Based on a saved value in the GI_Wellness Twon game instance (reflection scene number) we will pick a row of data to populate the reflection questions. This is a short term approach as going through the objective system is a bit complex right now. The row number will be updated after each scene and saved in the game instance.
  (bind _asgi_wellness_town (Utilities|Casting|CastToGI_WellnessTown (Game|GetGameInstance)))
  (bind _outrownames (DataTable|GetDataTableRowNames "/Game/DEV/Taylor/BP_Actors/RestAndReflect/DT_RestAndReflect-Questions+Answers.DT_RestAndReflect-Questions+Answers"))
  (bind _returnvalue (Utilities|GetDataTableRow "/Game/DEV/Taylor/BP_Actors/RestAndReflect/DT_RestAndReflect-Questions+Answers.DT_RestAndReflect-Questions+Answers" (Utilities|Array|Get(acopy) _outrownames (Variables|/Game/DEV/Taylor/GameInstance/GI_WellnessTown.GI_WellnessTown_C|GetReflectionSceneNumber _asgi_wellness_town)))
    (:then
      (Variables|Default|SetRowData _returnvalue))))

(event Collision|EventActorBeginOverlap
  (params (OtherActor :type Actor%20Object%20Reference)))

(event EventTick
  (params (DeltaSeconds :type Float%20%28single-precision%29)))

(fn ConstructionScript)

(fn GetDataforReflectionQuestions
  (return (Variables|Default|GetRowData)))